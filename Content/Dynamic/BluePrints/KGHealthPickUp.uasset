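; KGHealthPickUp is a health pickup that heals a KGCharacterBase character who overlaps it.
; On overlap it adds HealthOffering to the character's Health, capped at the Health value in that character's class defaults, which serves as the maximum.
; The pickup destroys itself after healing and stays in place when Health already equals that default.
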(event `self.ReceiveActorBeginOverlap`
  (params (OtherActor :type "Actor Object Reference"))
  ;[1 1 1] Health PickUp
  (bind _askgcharacter_base (cast `/Game/Dynamic/BluePrints/KGCharacterBase` OtherActor))
  (bind (_weapon _health) (defaults `Object` (`GameplayStatics.GetObjectClass` _askgcharacter_base)))
  (if (not (== _health (`/Game/Dynamic/BluePrints/KGCharacterBase.Health` _askgcharacter_base)))
    (set `/Game/Dynamic/BluePrints/KGCharacterBase.Health` (`KismetMathLibrary.FMin` (+ (`/Game/Dynamic/BluePrints/KGCharacterBase.Health` _askgcharacter_base) (`self.HealthOffering`)) _health) _askgcharacter_base)
    (`self.K2_DestroyActor`)))

(fn `UserConstructionScript`)