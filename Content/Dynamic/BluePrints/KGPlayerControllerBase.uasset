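; Base player controller for a cursor-aimed character, handling movement, jumping and melee input.
; Each tick it traces under the visible mouse cursor and turns the controlled pawn's yaw toward the hit point.
; Movement axes follow the camera's up and right vectors, so input is screen-relative rather than facing-relative.
; Jump requires a Character pawn, while melee plays the knight attack montage on a KGCharacterBase.
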(event `self.ReceiveBeginPlay`
  (set `self.bShowMouseCursor` true))

(event `self.ReceiveTick`
  (params (DeltaSeconds :type "Float (single-precision)"))
  (`self.ProcessMouse`))

(event `ProcessMouse`
  (bind (_hitresult _returnvalue) (`self.GetHitResultUnderCursorByChannel` "TraceTypeQuery1"))
  (bind _returnvalue_2 (`self.K2_GetPawn`))
  (bind (_returnvalue_roll _returnvalue_pitch _returnvalue_yaw) (`KismetMathLibrary.BreakRotator` (`KismetMathLibrary.Conv_VectorToRotator` (`KismetMathLibrary.GetDirectionUnitVector` (`self.K2_GetActorLocation` _returnvalue_2) (`.Location` (`GameplayStatics.BreakHitResult` _hitresult))))))
  ;[1 1 1] Character rotation with mouse
  (`/Engine/EditorBlueprintResources/StandardMacros.IsValid` (`self.K2_GetPawn`)
    (:`Is Valid`
      (if _returnvalue
        (`self.K2_SetActorRotation` _returnvalue_2 (`KismetMathLibrary.MakeRotator` 0.0 0.0 _returnvalue_yaw) false)))))

(event `InputAxis|Up`
  (params (AxisValue :type "Float (single-precision)"))
  (bind _returnvalue (`self.K2_GetPawn`))
  ;[1 1 1] Moving forward/backward
  (`/Engine/EditorBlueprintResources/StandardMacros.IsValid` _returnvalue
    (:`Is Valid`
      (`Pawn.AddMovementInput` _returnvalue (`SceneComponent.GetUpVector` (`PlayerCameraManager.TransformComponent` (`self.PlayerCameraManager`))) AxisValue false))))

(event `InputAxis|Right`
  (params (AxisValue :type "Float (single-precision)"))
  (bind _returnvalue (`self.K2_GetPawn`))
  ;[1 1 1] Mowing right/left
  (`/Engine/EditorBlueprintResources/StandardMacros.IsValid` _returnvalue
    (:`Is Valid`
      (`Pawn.AddMovementInput` _returnvalue (`SceneComponent.GetRightVector` (`PlayerCameraManager.TransformComponent` (`self.PlayerCameraManager`))) AxisValue false))))

(event `InputAction|Jump`
  (params (Key :type "Key Structure"))
  ;[1 1 1] Jumping
  (:`Pressed`
    (bind _ascharacter (cast `Character` (`self.K2_GetPawn`)))
    (`Character.Jump` _ascharacter)))

(event `InputAction|MeleeAttack`
  (params (Key :type "Key Structure"))
  (:`Pressed`
    (bind _askgcharacter_base (cast `/Game/Dynamic/BluePrints/KGCharacterBase` (`self.K2_GetPawn`)))
    (`Character.PlayAnimMontage` _askgcharacter_base "/Game/Static/Assets/Knight/KnightAttackMontage.KnightAttackMontage" 1.0 "None")))

(event `InputAction|MagicAttack`
  (params (Key :type "Key Structure")))

(fn `UserConstructionScript`)