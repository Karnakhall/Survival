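; Base AI controller that makes its pawn hunt and attack player-controlled KG characters, wandering when none is found.
; A looping timer from BeginPlay runs ProcessAI, which keeps a valid Target or finds one with a sphere overlap.
; It moves within the pawn's AttackRange and triggers its primary attack, otherwise moves to a random navigable point.
; A ForceJump event exists, but its timer is never hooked up.
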(event `ForceJump`
  (bind _returnvalue (`self.K2_GetPawn`))
  ;[1 1 1] Checking if character jump
  (`/Engine/EditorBlueprintResources/StandardMacros.IsValid` _returnvalue
    (:`Is Valid`
      (bind _ascharacter (cast `Character` _returnvalue))
      (`Character.Jump` _ascharacter))))

(event `ProcessAI`
  (bind _returnvalue (`self.K2_GetPawn`))
  ;[1 1 1] AI attack
  (`self.Target`
    (:`then`
      (`|AIMoveTo` _returnvalue (0.0 0.0 0.0) (`self.Target`) (`/Game/Dynamic/BluePrints/KGCharacterBase.AttackRange` (cast `/Game/Dynamic/BluePrints/KGCharacterBase` _returnvalue :!pure true)) :!label _label
        (:`OnSuccess`
          (bind _askgcharacter_base (cast `/Game/Dynamic/BluePrints/KGCharacterBase` (`self.K2_GetPawn`)))
          (`self.K2_SetFocalPoint` (`self.K2_GetActorLocation` (`self.Target`)))
          (`/Game/Dynamic/BluePrints/KGCharacterBase.UsePrimaryAttack` _askgcharacter_base))))
    (:`else`
      (bind _outactors (`KismetSystemLibrary.SphereOverlapActors` (`self.K2_GetActorLocation`) 1000.0 (`|MakeArray` "ObjectTypeQuery3" :!type "EObjectTypeQuery Enum") null (`|MakeArray` (`self.K2_GetPawn`) :!type "Actor Object Reference")))
      (for _array_element _outactors
        (bind _askgcharacter_base_2 (cast `/Game/Dynamic/BluePrints/KGCharacterBase` _array_element))
        (if (`self.IsPlayerController` (`Pawn.GetController` _askgcharacter_base_2))
          (set `self.Target` _askgcharacter_base_2)
          (break)))
      (`self.Target`
        (:`then`
          (goto _label))
        (:`else`
          (`self.Wander`))))))

(event `self.ReceiveBeginPlay`
  ;[1 1 1] Simple AI Controller
  (`KismetSystemLibrary.K2_SetTimerDelegate` (delegate `ProcessAI`) 2.0 true))

(event `Wander`
  (bind _returnvalue (`self.K2_GetPawn`))
  ;[1 1 1] Simple AI Controller
  (`/Engine/EditorBlueprintResources/StandardMacros.IsValid` _returnvalue
    (:`Is Valid`
      (`|AIMoveTo` _returnvalue (`NavigationSystemV1.K2_GetRandomLocationInNavigableRadius` (`self.K2_GetActorLocation` _returnvalue) 2000.0 null null) null))))

(fn `UserConstructionScript`)