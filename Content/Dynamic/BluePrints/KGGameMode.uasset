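; Game mode that runs wave-based enemy spawning, starting at the first wave on BeginPlay.
; Each wave's class list is shuffled into a queue, which a looping timer drains by spawning AI at random PlayerStarts.
; When a spawned pawn is destroyed with the queue empty and no KGAIControllerBase left, the next wave begins.
; Dispatchers announce new waves and game end; after the last wave, the view blends to a random CameraActor.
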(event `self.ReceiveBeginPlay`
  ;[1 1 1] Spawn Enemy
  (`KismetSystemLibrary.K2_SetTimerDelegate` (delegate `SpawnEnemy`) 1.0 true)
  (`self.ResetGame`))

(event `SpawnEnemy`
  ;[1 1 1] Spawn Enemy
  (if (> (`KismetArrayLibrary.Array_Length` (`self.Queue`)) 0)
    (bind _outactors (`GameplayStatics.GetAllActorsOfClass` "/Script/Engine.PlayerStart"))
    (bind _output (`|GetArrayItem` _outactors (`KismetMathLibrary.RandomInteger` (`KismetArrayLibrary.Array_Length` _outactors))))
    (bind _returnvalue (`AIBlueprintHelperLibrary.SpawnAIFromClass` (`|GetArrayItem` (`self.Queue`)) null (`self.K2_GetActorLocation` _output) (`self.K2_GetActorRotation` _output) false null))
    (`KismetArrayLibrary.Array_Remove` (`self.Queue`))
    (add `self.OnDestroyed` _returnvalue (delegate `CheckWaveComplete`))))

(event `CheckWaveComplete` :!signature `self.OnDestroyed`
  (params (DestroyedActor :type "Actor Object Reference"))
  ;[1 1 1] Spawn Enemy
  ;;[1 1 1] Check If The Wave Is Over And Start New Wave
  (if (== (`KismetArrayLibrary.Array_Length` (`self.Queue`)) 0)
    (bind _outactors (`GameplayStatics.GetAllActorsOfClass` "/Game/Dynamic/BluePrints/KGAIControllerBase.KGAIControllerBase_C"))
    (if (== (`KismetArrayLibrary.Array_Length` _outactors) 0)
      (`self.StartNewWave`))))

(event `ResetGame`
  (bind _output_classtospawn (break `/Game/Dynamic/BluePrints/BP_WaveStruct` (`|GetArrayItem` (`self.Waves`) (`self.WaveIndex`))))
  (set `self.WaveIndex` 0)
  ;[1 1 1] SpawnWavesOfEnemy
  (bind _output_get (set `self.Queue` _output_classtospawn :!label _label))
  (`KismetArrayLibrary.Array_Shuffle` _output_get))

(event `StartNewWave`
  ;[1 1 1] SpawnWavesOfEnemy
  (`/Engine/EditorBlueprintResources/StandardMacros.IncrementInt` (`self.WaveIndex`)
    (:`  `
      (`self.NewWave`)
      (if (< (`KismetArrayLibrary.Array_LastIndex` (`self.Waves`)) (`self.WaveIndex`))
        (`self.EndGame`)
        (else
          (goto _label))))))

(event `EndGame`
  (`self.EndGameDispatcher`)
  (bind _outactors (`GameplayStatics.GetAllActorsOfClass` "/Script/Engine.CameraActor"))
  (`PlayerController.SetViewTargetWithBlend` (`GameplayStatics.GetPlayerController` 0) (`|GetArrayItem` _outactors (`KismetMathLibrary.RandomInteger` (`KismetArrayLibrary.Array_Length` _outactors))) 4.0 "VTBlend_Linear" 0.0 true))

(fn `UserConstructionScript`)